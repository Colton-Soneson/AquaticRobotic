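; BP_BoatAI is an AI boat whose cannon repeatedly fires projectiles, apparently intended to target the player.
; Each Tick it sets the cannon's rotation from the BP_RDPlayer camera's absolute world location used as an X vector, not the cannon-to-player direction.
; A Delay on Tick paces FirstPersonProjectile spawns at the Sphere component using the cannon's rotation.
; The cannon sound node is unconnected, with a timing TODO.
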(event EventTick
  (params (DeltaSeconds :type Float%20%28single-precision%29))
  (bind _cannon (Variables|Default|GetCannon))
  (Utilities|FlowControl|Sequence
    (:then_0
      (bind _returnvalue (Actor|GetActorOfClass "/Game/RoboticAcquatic/CustomBP/BP_RDPlayer.BP_RDPlayer_C"))
      (Transformation|SetWorldRotation _cannon (Math|Conversions|RotationFromXVector (Transformation|GetWorldLocation (Variables|/Game/RoboticAcquatic/CustomBP/BP_RDPlayer.BP_RDPlayer_C|GetCamera _returnvalue))) false false))
    (:then_1
      (Utilities|FlowControl|Delay (Variables|Default|GetCannon%20Fire%20Delay))
      (Game|SpawnActorfromClass "/Game/RoboticAcquatic/CustomBP/FirstPersonProjectile.FirstPersonProjectile_C" (Math|Transform|MakeTransform (Transformation|GetWorldLocation (Variables|Default|GetSphere)) (Transformation|GetWorldRotation _cannon)) "AdjustIfPossibleButDontSpawnIfColliding" 0 0))))

(fn ConstructionScript)